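; Nightlight actor that serves as the win goal, lighting up once the player has collected enough batteries.
; Tick casts the player pawn to BP_ThirdPersonCharacter and arms NightlightOn when BatteriesCollected reaches four or more.
; While armed, any Box begin-overlap shows the PointLight and sets the player character's GameWon flag, without checking which actor overlapped.
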(event `self.Box.OnComponentBeginOverlap`
  (params (OverlappedComponent :type "PrimitiveComponent Object Reference") (OtherActor :type "Actor Object Reference") (OtherComp :type "PrimitiveComponent Object Reference") (OtherBodyIndex :type Integer) (bFromSweep :type Boolean) (SweepResult :type "HitResult Structure (by ref)"))
  ;[1 0.2181 0.05805] Light On Overlap
  (if (`self.nightlight on`)
    (`SceneComponent.SetVisibility` (`self.PointLight`) true false)
    ;[0.4683 1 0.5093] Win Condition
    (bind _asbp_third_person_character (cast `/Game/ThirdPerson/Blueprints/BP_ThirdPersonCharacter` (`GameplayStatics.GetPlayerPawn` 0)))
    (set `/Game/ThirdPerson/Blueprints/BP_ThirdPersonCharacter.GameWon` true _asbp_third_person_character)))

(event `self.ReceiveTick`
  (params (DeltaSeconds :type "Float (single-precision)"))
  ;[1 0.8427 0.4836] Battery Light Condition
  (bind _asbp_third_person_character (cast `/Game/ThirdPerson/Blueprints/BP_ThirdPersonCharacter` (`GameplayStatics.GetPlayerPawn` 0)))
  (if (>= (`/Game/ThirdPerson/Blueprints/BP_ThirdPersonCharacter.BatteriesCollected` _asbp_third_person_character) 4)
    (set `self.nightlight on` true)))

(fn `UserConstructionScript`)